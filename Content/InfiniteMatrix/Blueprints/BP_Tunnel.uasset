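; Tunnel segment for an endless obstacle run, with a rotating holed wall and child-actor health pack and enemy.
; Passing its trigger has TunnelSpawner spawn another tunnel, destroys this one and increments the player's WallsPassed.
; Hitting the wall cuts health with shake, sound and damage widget, showing restart on death.
; BeginPlay randomly culls the pickup and sometimes enemy; uncalled-here helpers randomize wall mesh, roll and child placement.
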(event OnComponentBeginOverlap(TriggerZone)
  (params (OverlappedComponent :type Primitive%20Component%20Object%20Reference) (OtherActor :type Actor%20Object%20Reference) (OtherComp :type Primitive%20Component%20Object%20Reference) (OtherBodyIndex :type Integer) (bFromSweep :type Boolean) (SweepResult :type Hit%20Result%20Structure%20%28by%20ref%29))
  (Utilities|Casting|CastToBP_Player OtherActor)
  (Default|SpawnTunnelatSpawnPoint (Variables|Default|GetTunnelSpawner))
  (Actor|DestroyActor)
  ;[1 1 1] WallsPassed
  (bind _asbp_player (Utilities|Casting|CastToBP_Player OtherActor))
  (Variables|/Game/InfiniteMatrix/Blueprints/BP_Player.BP_Player_C|SetWallsPassed _asbp_player (+ 1 (Variables|/Game/InfiniteMatrix/Blueprints/BP_Player.BP_Player_C|GetWallsPassed _asbp_player))))

(event OnComponentBeginOverlap(WallMesh)
  (params (OverlappedComponent :type Primitive%20Component%20Object%20Reference) (OtherActor :type Actor%20Object%20Reference) (OtherComp :type Primitive%20Component%20Object%20Reference) (OtherBodyIndex :type Integer) (bFromSweep :type Boolean) (SweepResult :type Hit%20Result%20Structure%20%28by%20ref%29))
  (bind _asbp_player (Utilities|Casting|CastToBP_Player OtherActor))
  (CallFunction|DecraseHealth _asbp_player)
  (Class|LegacyCameraShake|StartLegacyCameraShake (Game|GetPlayerCameraManager 0) "/Game/InfiniteMatrix/Blueprints/BP_CameraShake.BP_CameraShake_C" 1.0 "CameraLocal" "0, 0, 0")
  (bind _returnvalue (UserInterface|CreateWidget "/Game/InfiniteMatrix/UI/WBP_DMGIndicator.WBP_DMGIndicator_C"))
  (UserInterface|Viewport|AddtoViewport _returnvalue 0)
  (Audio|PlaySound2D "/Engine/EditorSounds/Notifications/CompileFailed.CompileFailed" 1.0 1.0 0.0 0 0))

(event EventBeginPlay
  (bind _outactors (Actor|GetAllActorsOfClass "/Game/InfiniteMatrix/Blueprints/BP_Player.BP_Player_C"))
  (Variables|Default|SetPlayerReference (Utilities|Array|Get(acopy) _outactors))
  (CallFunction|RemoveHealthPack))

(event EventTick
  (params (DeltaSeconds :type Float%20%28single-precision%29))
  (Transformation|AddLocalRotation (Variables|Default|GetWallMesh) (Math|Rotator|MakeRotator (* DeltaSeconds (Variables|Default|GetRotateSpeed)) 0.0 0.0) false false))

(fn ConstructionScript)

(fn RandomizeWall
  (Components|StaticMesh|SetStaticMesh (Variables|Default|GetWallMesh) (Utilities|Select :Index (Math|Random|RandomIntegerinRange 0 3) :Option%200 "/Game/InfiniteMatrix/Meshes/SM_Hole_01.SM_Hole_01" :Option%201 "/Game/InfiniteMatrix/Meshes/SM_Hole_02.SM_Hole_02" :Option%202 "/Game/InfiniteMatrix/Meshes/SM_Hole_03.SM_Hole_03" :Option%203 0))
  (Transformation|AddLocalRotation (Variables|Default|GetWallMesh) (Math|Rotator|MakeRotator (Math|Random|RandomFloatinRange 0.0 3.6e+02) 0.0 0.0) false false))

(fn RandomizeHPLocation
  (Transformation|AddLocalOffset (Variables|Default|GetBP_HealthPack) (Math|Vector|MakeVector (Math|Random|RandomFloatinRange -1e+02 1e+02) (Math|Random|RandomFloatinRange -175.0 175.0) (Math|Random|RandomFloatinRange -175.0 175.0)) false true))

(fn RemoveHealthPack
  (if (not (== 1 (Math|Random|RandomIntegerinRange 0 5)))
    (Actor|DestroyActor (Variables|/Script/Engine.ChildActorComponent|GetChildActor (Variables|Default|GetBP_HealthPack)))
    (if (== 1 (Math|Random|RandomIntegerinRange 0 2))
      (Actor|DestroyActor (Variables|/Script/Engine.ChildActorComponent|GetChildActor (Variables|Default|GetBP_Enemy))))))

(fn RandomizeEnemyLocation
  (Transformation|AddLocalOffset (Variables|Default|GetBP_Enemy) (Math|Vector|MakeVector (Math|Random|RandomFloatinRange -1e+02 1e+02) (Math|Random|RandomFloatinRange -175.0 175.0) (Math|Random|RandomFloatinRange -175.0 175.0)) false true))

(fn DecraseHealth
  (params (PlayerRef :type BP%20Player%20Object%20Reference))
  (bind _playerreference (Variables|Default|GetPlayerReference))
  (Variables|/Game/InfiniteMatrix/Blueprints/BP_Player.BP_Player_C|SetPlayerHealth PlayerRef (select (> (Variables|/Game/InfiniteMatrix/Blueprints/BP_Player.BP_Player_C|GetPlayerHealth (Variables|Default|GetPlayerReference)) 1) (- (Variables|/Game/InfiniteMatrix/Blueprints/BP_Player.BP_Player_C|GetPlayerHealth (Variables|Default|GetPlayerReference)) 33) (- (Variables|/Game/InfiniteMatrix/Blueprints/BP_Player.BP_Player_C|GetPlayerHealth (Variables|Default|GetPlayerReference)) 1)))
  (if (not (> (Variables|/Game/InfiniteMatrix/Blueprints/BP_Player.BP_Player_C|GetPlayerHealth (Variables|Default|GetPlayerReference)) 0))
    (Variables|/Game/InfiniteMatrix/Blueprints/BP_Player.BP_Player_C|SetIsDead _playerreference true)
    (Default|DisplayRestart _playerreference)))