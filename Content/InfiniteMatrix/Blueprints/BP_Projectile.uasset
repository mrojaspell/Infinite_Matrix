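; BP_Projectile is a projectile that ties its speed to the player and removes itself on impact or when its lifespan runs out.
; On BeginPlay it finds the first BP_Player and sets the movement component's InitialSpeed to that player's ForwardSpeed plus a fixed boost.
; Tick counts down the lifespan to destruction.
; Hitbox overlap with anything other than the player also destroys it, with no damage logic here.
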(event OnComponentBeginOverlap(Hitbox)
  (params (OverlappedComponent :type Primitive%20Component%20Object%20Reference) (OtherActor :type Actor%20Object%20Reference) (OtherComp :type Primitive%20Component%20Object%20Reference) (OtherBodyIndex :type Integer) (bFromSweep :type Boolean) (SweepResult :type Hit%20Result%20Structure%20%28by%20ref%29))
  (Utilities|Casting|CastToBP_Player OtherActor
    (:CastFailed
      (Actor|DestroyActor))))

(event EventBeginPlay
  (bind _outactors (Actor|GetAllActorsOfClass "/Game/InfiniteMatrix/Blueprints/BP_Player.BP_Player_C"))
  (bind _output_get (Variables|Default|SetPlayerRef (Utilities|Array|Get(acopy) _outactors)))
  (Variables|/Script/Engine.ProjectileMovementComponent|SetInitialSpeed (Variables|Default|GetProjectileMovement) (+ (Variables|/Game/InfiniteMatrix/Blueprints/BP_Player.BP_Player_C|GetForwardSpeed _output_get) 2.5e+03)))

(event Collision|EventActorBeginOverlap
  (params (OtherActor :type Actor%20Object%20Reference)))

(event EventTick
  (params (DeltaSeconds :type Float%20%28single-precision%29))
  (Variables|Default|SetProjectileLifespan (- (Variables|Default|GetProjectileLifespan) DeltaSeconds))
  (if (<= (Variables|Default|GetProjectileLifespan) 0.0)
    (Actor|DestroyActor)))

(fn ConstructionScript)