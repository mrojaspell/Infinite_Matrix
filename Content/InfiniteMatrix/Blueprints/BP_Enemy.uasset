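; BP_Enemy is an enemy actor that damages the player on contact and awards score when hit by a projectile.
; Its collision overlap either lowers player health with camera shake, damage widget and sound, or raises the kill count and score, destroying itself in both cases.
; It writes to a player reference cached at BeginPlay, triggering the restart display on death and scaling each kill's points by total enemies destroyed.
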(event OnComponentBeginOverlap(CollisionBox)
  (params (OverlappedComponent :type Primitive%20Component%20Object%20Reference) (OtherActor :type Actor%20Object%20Reference) (OtherComp :type Primitive%20Component%20Object%20Reference) (OtherBodyIndex :type Integer) (bFromSweep :type Boolean) (SweepResult :type Hit%20Result%20Structure%20%28by%20ref%29))
  (bind _asbp_player (Utilities|Casting|CastToBP_Player OtherActor)
    (:then
      (CallFunction|DecreaseHealth _asbp_player)
      (Class|LegacyCameraShake|StartLegacyCameraShake (Game|GetPlayerCameraManager 0) "/Game/InfiniteMatrix/Blueprints/BP_CameraShake.BP_CameraShake_C" 1.0 "CameraLocal" "0, 0, 0")
      (bind _returnvalue (UserInterface|CreateWidget "/Game/InfiniteMatrix/UI/WBP_DMGIndicator.WBP_DMGIndicator_C"))
      (UserInterface|Viewport|AddtoViewport _returnvalue 0)
      (Audio|PlaySound2D "/Engine/EditorSounds/Notifications/CompileFailed.CompileFailed" 1.0 1.0 0.0 0 0))
    (:CastFailed
      (Utilities|Casting|CastToBP_Projectile OtherActor)
      (CallFunction|IncreaseScore)
      (Audio|PlaySound2D "/Engine/VREditor/Sounds/UI/Laser_Push.Laser_Push" 1.0 1.0 0.0 0 0)))
  (Actor|DestroyActor))

(event EventBeginPlay
  (bind _outactors (Actor|GetAllActorsOfClass "/Game/InfiniteMatrix/Blueprints/BP_Player.BP_Player_C"))
  (Variables|Default|SetPlayerReference (Utilities|Array|Get(acopy) _outactors)))

(event Collision|EventActorBeginOverlap
  (params (OtherActor :type Actor%20Object%20Reference)))

(event EventTick
  (params (DeltaSeconds :type Float%20%28single-precision%29)))

(fn ConstructionScript)

(fn DecreaseHealth
  (params (PlayerRef :type BP%20Player%20Object%20Reference))
  (bind _playerreference (Variables|Default|GetPlayerReference))
  (Variables|/Game/InfiniteMatrix/Blueprints/BP_Player.BP_Player_C|SetPlayerHealth PlayerRef (select (> (Variables|/Game/InfiniteMatrix/Blueprints/BP_Player.BP_Player_C|GetPlayerHealth (Variables|Default|GetPlayerReference)) 1) (- (Variables|/Game/InfiniteMatrix/Blueprints/BP_Player.BP_Player_C|GetPlayerHealth (Variables|Default|GetPlayerReference)) 33) (- (Variables|/Game/InfiniteMatrix/Blueprints/BP_Player.BP_Player_C|GetPlayerHealth (Variables|Default|GetPlayerReference)) 1)))
  (if (not (> (Variables|/Game/InfiniteMatrix/Blueprints/BP_Player.BP_Player_C|GetPlayerHealth (Variables|Default|GetPlayerReference)) 0))
    (Variables|/Game/InfiniteMatrix/Blueprints/BP_Player.BP_Player_C|SetIsDead _playerreference true)
    (Default|DisplayRestart _playerreference)))

(fn IncreaseScore
  (bind _playerreference (Variables|Default|GetPlayerReference))
  (bind _playerreference_2 (Variables|Default|GetPlayerReference))
  (Variables|/Game/InfiniteMatrix/Blueprints/BP_Player.BP_Player_C|SetEnemiesDestroyed _playerreference (+ (Variables|/Game/InfiniteMatrix/Blueprints/BP_Player.BP_Player_C|GetEnemiesDestroyed _playerreference) 1))
  (Variables|/Game/InfiniteMatrix/Blueprints/BP_Player.BP_Player_C|SetScore _playerreference_2 (+ (Variables|/Game/InfiniteMatrix/Blueprints/BP_Player.BP_Player_C|GetScore _playerreference_2) (* (Variables|/Game/InfiniteMatrix/Blueprints/BP_Player.BP_Player_C|GetEnemiesDestroyed _playerreference_2) 1000))))